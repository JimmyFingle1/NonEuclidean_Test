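; Portal actor that shows a live view through its linked portal on a plane mesh.
; After a short delay at BeginPlay, it renders the linked portal's scene capture camera into a viewport-sized render target fed to a dynamic material.
; Each tick, ticking post-update, it mirrors the player camera's transform into the linked portal's space to position that capture camera.
; A clip plane just behind its own surface keeps its capture camera from clipping.
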(event EventBeginPlay
  (bind _returnvalue (Viewport|GetViewportSize))
  ;[0.15 0.15 0.15 0.5] Comment
  (Utilities|FlowControl|Delay 1.0)
  (Components|Tick|SetTickGroup "TG_PostUpdateWork")
  (bind _returnvalue_2 (Rendering|Material|CreateDynamicMaterialInstance "/Game/JPContent/PortalSystem/Portal_MAT.Portal_MAT" "None" "None" :!class /Script/Engine.KismetMaterialLibrary))
  (bind _output_get (Variables|Default|SetPortal_MAT _returnvalue_2))
  (Rendering|Material|SetMaterial (Variables|Default|GetPortalPlane) 0 _output_get)
  (bind _returnvalue_3 (Rendering|CreateRenderTarget2D (Math|Float|Truncate (.x _returnvalue)) (Math|Float|Truncate (.y _returnvalue)) "RTF_RGBA16f"))
  (bind _output_get_2 (Variables|Default|SetPortal_RT _returnvalue_3))
  (Rendering|Material|SetTextureParameterValue (Variables|Default|GetPortal_MAT) "Texture" _output_get_2)
  (Variables|/Script/Engine.SceneCaptureComponent2D|SetTextureTarget (Variables|Portal_BP_C|GetPortalCamera (Variables|Default|GetLinkedPortal)) (Variables|Default|GetPortal_RT))
  (CallFunction|SetClipPlanes))

(event Collision|EventActorBeginOverlap
  (params (OtherActor :type Actor%20Object%20Reference)))

(event EventTick
  (params (DeltaSeconds :type Float%20%28single-precision%29))
  (CallFunction|UpdateSceneCapture))

(fn ConstructionScript)

(fn UpdateSceneCapture
  (bind _returnvalue (Transformation|GetActorTransform))
  (bind _returnvalue_2 (Game|GetPlayerCameraManager 0))
  (bind _returnvalue_3 (Transformation|GetActorTransform))
  (bind _linkedportal (Variables|Default|GetLinkedPortal))
  (bind _returnvalue_4 (Transformation|GetActorTransform _linkedportal))
  (bind (_location _rotation _scale) (Math|Transform|BreakTransform _returnvalue))
  (bind _transformcomponent (Variables|/Script/Engine.PlayerCameraManager|GetTransformComponent _returnvalue_2))
  (bind _returnvalue_5 (Transformation|GetWorldRotation _transformcomponent))
  (bind (_x _y _z) (Math|Vector|BreakVector _scale))
  (bind (_x_2 _y_2 _z_2) (Math|Rotator|BreakRotIntoAxes _returnvalue_5))
  (Transformation|SetWorldLocationAndRotation (Variables|Portal_BP_C|GetPortalCamera (Variables|Default|GetLinkedPortal)) (Math|Transform|TransformLocation (Transformation|GetActorTransform (Variables|Default|GetLinkedPortal)) (Math|Transform|InverseTransformLocation (Math|Transform|MakeTransform _location _rotation (Math|Vector|MakeVector (* _x -1.0) (* _y -1.0) _z)) (Transformation|GetWorldLocation (Variables|/Script/Engine.PlayerCameraManager|GetTransformComponent (Game|GetPlayerCameraManager 0))))) (Math|Rotator|MakeRotationfromAxes (Math|Transform|TransformDirection _returnvalue_4 (Math|Vector|MirrorVectorbyNormal (Math|Vector|MirrorVectorbyNormal (Math|Transform|InverseTransformDirection _returnvalue_3 _x_2) "1.000000,0.000000,0.000000") "0.000000,1.000000,0.000000")) (Math|Transform|TransformDirection _returnvalue_4 (Math|Vector|MirrorVectorbyNormal (Math|Vector|MirrorVectorbyNormal (Math|Transform|InverseTransformDirection _returnvalue_3 _y_2) "1.000000,0.000000,0.000000") "0.000000,1.000000,0.000000")) (Math|Transform|TransformDirection _returnvalue_4 (Math|Vector|MirrorVectorbyNormal (Math|Vector|MirrorVectorbyNormal (Math|Transform|InverseTransformDirection _returnvalue_3 _z_2) "1.000000,0.000000,0.000000") "0.000000,1.000000,0.000000"))) false false))

(fn SetClipPlanes
  (bind _portalcamera (Variables|Default|GetPortalCamera))
  ;[0.15 0.15 0.15 0.5] Stop camera from clipping
  (Utilities|IsValid (Variables|Default|GetLinkedPortal)
    (:Is%20Valid
      (Variables|/Script/Engine.SceneCaptureComponent2D|SetbEnableClipPlane _portalcamera true)
      (Variables|/Script/Engine.SceneCaptureComponent2D|SetClipPlaneBase _portalcamera (+ (Transformation|GetWorldLocation (Variables|Default|GetPortalPlane)) (* (Math|Vector|GetForwardVector (Variables|Default|GetForwardDirection)) -3.0)))
      (Variables|/Script/Engine.SceneCaptureComponent2D|SetClipPlaneNormal _portalcamera (Math|Vector|GetForwardVector (Variables|Default|GetForwardDirection))))))