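; BP_SeemlessTeleport is an actor that seamlessly teleports player 0's character from an Enterance box to an Exit box on overlap.
; The character's transform is re-expressed relative to Enterance and applied from Exit, preserving offset and orientation.
; Control rotation and velocity are rotated from Enterance space into Exit space the same way, keeping view and momentum continuous.
; The construction script gives both boxes the same BoxSize extent.
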(event OnComponentBeginOverlap(Enterance)
  (params (OverlappedComponent :type Primitive%20Component%20Object%20Reference) (OtherActor :type Actor%20Object%20Reference) (OtherComp :type Primitive%20Component%20Object%20Reference) (OtherBodyIndex :type Integer) (bFromSweep :type Boolean) (SweepResult :type Hit%20Result%20Structure%20%28by%20ref%29))
  (if (== OtherActor (Game|GetPlayerCharacter 0))
    (Transformation|SetActorTransform (Game|GetPlayerCharacter 0) (CallFunction|GetDestinationTransfrom))
    (Pawn|SetControlRotation (Game|GetPlayerController 0) (CallFunction|GetControlRotation))
    (Variables|/Script/Engine.MovementComponent|SetVelocity (Pawn|GetMovementComponent (Game|GetPlayerCharacter 0)) (CallFunction|GetDestinationVelocity))))

(fn ConstructionScript
  (Components|Box|SetBoxExtent (Variables|Default|GetEnterance) (Variables|Default|GetBoxSize) true))

(fn GetDestinationTransfrom
  (return (Math|Transform|ComposeTransforms (Math|Transform|MakeRelativeTransform (Transformation|GetActorTransform (Game|GetPlayerCharacter 0)) (Transformation|GetWorldTransform (Variables|Default|GetEnterance))) (Transformation|GetWorldTransform (Variables|Default|GetExit)))))

(fn GetControlRotation
  (return (Math|Rotator|MakeRotfromX (Math|Vector|RotateVector (Math|Vector|UnrotateVector (Math|Vector|GetForwardVector (Pawn|GetControlRotation (Game|GetPlayerController 0) :!class /Script/Engine.Controller)) (Transformation|GetWorldRotation (Variables|Default|GetEnterance))) (Transformation|GetWorldRotation (Variables|Default|GetExit))))))

(fn GetDestinationVelocity
  (return (Math|Vector|RotateVector (Math|Vector|UnrotateVector (Variables|/Script/Engine.MovementComponent|GetVelocity (Pawn|GetMovementComponent (Game|GetPlayerCharacter 0))) (Transformation|GetWorldRotation (Variables|Default|GetEnterance))) (Transformation|GetWorldRotation (Variables|Default|GetExit)))))