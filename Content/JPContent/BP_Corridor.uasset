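; BP_Corridor is a self-replicating corridor segment that builds an endless hallway around the first-person player as they move along it.
; Overlap triggers spawn another corridor at the forward arrow or destroy this segment as the player passes.
; A reverse pair does the same only when the player's X velocity is negative, spawning at the reverse arrow with a fixed X offset.
; Tick prints that X velocity, apparently for debugging.
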(event OnComponentBeginOverlap(SpawnCollision)
  (params (OverlappedComponent :type Primitive%20Component%20Object%20Reference) (OtherActor :type Actor%20Object%20Reference) (OtherComp :type Primitive%20Component%20Object%20Reference) (OtherBodyIndex :type Integer) (bFromSweep :type Boolean) (SweepResult :type Hit%20Result%20Structure%20%28by%20ref%29))
  ;[0.15 0.15 0.15 0.5] Spawns next corridor
  (if (== OtherActor (Variables|Default|GetChar%20Ref))
    (Game|SpawnActorfromClass "BP_Corridor_C" (Math|Transform|MakeTransform (Transformation|GetWorldLocation (Variables|Default|GetArrow)) "0, 0, 0" "1.000000,1.000000,1.000000") "Undefined" "MultiplyWithRoot" 0 0)))

(event OnComponentBeginOverlap(DeleteCollision)
  (params (OverlappedComponent :type Primitive%20Component%20Object%20Reference) (OtherActor :type Actor%20Object%20Reference) (OtherComp :type Primitive%20Component%20Object%20Reference) (OtherBodyIndex :type Integer) (bFromSweep :type Boolean) (SweepResult :type Hit%20Result%20Structure%20%28by%20ref%29))
  ;[0.15 0.15 0.15 0.5] Deletes self
  (if (== OtherActor (Variables|Default|GetChar%20Ref))
    (Actor|DestroyActor)))

(event OnComponentBeginOverlap(SpawnReverseCollision)
  (params (OverlappedComponent :type Primitive%20Component%20Object%20Reference) (OtherActor :type Actor%20Object%20Reference) (OtherComp :type Primitive%20Component%20Object%20Reference) (OtherBodyIndex :type Integer) (bFromSweep :type Boolean) (SweepResult :type Hit%20Result%20Structure%20%28by%20ref%29))
  (bind _char_ref (Variables|Default|GetChar%20Ref))
  ;[0.15 0.15 0.15 0.5] Spawn reverse corridor
  (if (and (== OtherActor _char_ref) (< (.x (Transformation|GetComponentVelocity (Variables|/Script/Engine.Character|GetCapsuleComponent _char_ref))) 0.0))
    (Game|SpawnActorfromClass "BP_Corridor_C" (Math|Transform|MakeTransform (+ (Transformation|GetWorldLocation (Variables|Default|GetArrowReverse)) "1500.000000,0.000000,0.000000") "0, 0, 0" "1.000000,1.000000,1.000000") "Undefined" "MultiplyWithRoot" 0 0)))

(event OnComponentBeginOverlap(DeleteReverseCollision)
  (params (OverlappedComponent :type Primitive%20Component%20Object%20Reference) (OtherActor :type Actor%20Object%20Reference) (OtherComp :type Primitive%20Component%20Object%20Reference) (OtherBodyIndex :type Integer) (bFromSweep :type Boolean) (SweepResult :type Hit%20Result%20Structure%20%28by%20ref%29))
  (bind _char_ref (Variables|Default|GetChar%20Ref))
  ;[0.15 0.15 0.15 0.5] Delete self if reverse
  (if (and (== OtherActor _char_ref) (< (.x (Transformation|GetComponentVelocity (Variables|/Script/Engine.Character|GetCapsuleComponent _char_ref))) 0.0))
    (Actor|DestroyActor)))

(event EventBeginPlay
  ;[0.15 0.15 0.15 0.5] Setting character reference
  (bind _asbp_first_person_character (Utilities|Casting|CastToBP_FirstPersonCharacter (Game|GetPlayerCharacter 0)))
  (Variables|Default|SetChar%20Ref _asbp_first_person_character))

(event EventTick
  (params (DeltaSeconds :type Float%20%28single-precision%29))
  (Development|PrintString (Utilities|String|ToString(Float) (.x (Transformation|GetComponentVelocity (Variables|/Script/Engine.Character|GetCapsuleComponent (Variables|Default|GetChar%20Ref)))))))

(fn ConstructionScript)